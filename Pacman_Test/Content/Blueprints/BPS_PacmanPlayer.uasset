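; BPS_PacmanPlayer is an unfinished Pac-Man player character prototype built around grid-based movement.
; MoveUpGrid proposes the next Y cell and asks CustomGridCoordEvent to validate it, but that stub always returns false, so the move reverts.
; Unconnected EventGraph fragments hold experiments with four-direction velocity, timeline movement and a flattened-array tile lookup using a 22-wide index.
; No events drive the graph and the construction script is empty.
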(event Input|ActionEvents|InputActionWKey
  (params (Key :type Key%20Structure)))

(event Input|ActionEvents|InputActionSKey
  (params (Key :type Key%20Structure)))

(event Input|ActionEvents|InputActionAKey
  (params (Key :type Key%20Structure)))

(event Input|ActionEvents|InputActionDKey
  (params (Key :type Key%20Structure)))

(fn ConstructionScript)

(fn MoveUpGrid
  (Variables|Default|SetNextGridCoord (Math|Vector|MakeVector (.x (Variables|Default|GetCurrentGridCoord)) (+ (.y (Variables|Default|GetCurrentGridCoord)) 1.0) (.z (Variables|Default|GetCurrentGridCoord))))
  (bind _canmove (CallFunction|CustomGridCoordEvent (Variables|Default|GetNextGridCoord)))
  (if _canmove
    (Variables|Default|SetCurrentGridCoord (Variables|Default|GetNextGridCoord))
    (Development|PrintString "a")
    (else
      (Variables|Default|SetNextGridCoord (Variables|Default|GetCurrentGridCoord))
      (Development|PrintString "b"))))

(fn CustomGridCoordEvent
  (params (PlayerGridCoord :type Vector :default "0, 0, 0"))
  (return false))